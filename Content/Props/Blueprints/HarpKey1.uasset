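; Harp puzzle prop where the player plays a note sequence on keys 1–7 to match a Solution string.
; Box1 overlap toggles help text and actor input; E switches between the harp view and the player character, disabling character input meanwhile.
; Each key plays a sound, appends its note letter and briefly flashes KeepPlaying.
; At full length, a match sets Solved, plays Success and restores player control, while a mismatch clears the attempt.
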(event `Key|One`
  (bind _keep_playing_ (`self.Keep Playing!`))
  ;[1 1 1] Checking Strings
  (:`Pressed`
    (`GameplayStatics.PlaySoundAttached` "/Game/Props/Blueprints/1.1" (`self.String1`))
    (if (`KismetStringLibrary.EqualEqual_StrStr` (`self.Solution`) (`self.PlaySolution`))
      (set `self.Solved?` true)
      (else
        (set `self.PlaySolution` (`KismetStringLibrary.Concat_StrStr` (`self.PlaySolution`) (`self.C`)))
        (`SceneComponent.ToggleVisibility` _keep_playing_ false)
        (`KismetSystemLibrary.Delay` 0.5)
        (`SceneComponent.ToggleVisibility` _keep_playing_ false)
        (if (== (`KismetStringLibrary.Len` (`self.Solution`)) (`KismetStringLibrary.Len` (`self.PlaySolution`))) :!label _label
          (if (`KismetStringLibrary.EqualEqual_StrStr` (`self.Solution`) (`self.PlaySolution`))
            (`GameplayStatics.PlaySoundAttached` "/Game/Props/Blueprints/Success.Success" (`self.HarpControl`))
            (set `self.Solved?` true)
            ;[1 1 1] Harp Input
            (`PlayerController.SetViewTargetWithBlend` (`GameplayStatics.GetPlayerController` 0) (`GameplayStatics.GetPlayerCharacter` 0) 0.0 "VTBlend_Linear" 0.0 false :!label _label_2)
            (`self.EnableInput` (`GameplayStatics.GetPlayerCharacter` 0) (`GameplayStatics.GetPlayerController` 0))
            (else
              (set `self.PlaySolution` ""))))))))

(event `Key|E`
  ;[1 1 1] Harp Input
  (:`Pressed`
    (if (`self.Solving?`)
      (set `self.Solving?` false)
      (goto _label_2)
      (else
        (set `self.Solving?` true)
        (set `self.bFindCameraComponentWhenViewTarget` (`self.bFindCameraComponentWhenViewTarget`))
        (`self.DisableInput` (`GameplayStatics.GetPlayerCharacter` 0) (`GameplayStatics.GetPlayerController` 0))
        (`PlayerController.SetViewTargetWithBlend` (`GameplayStatics.GetPlayerController` 0) self 0.0 "VTBlend_Linear" 0.0 true)))))

(event `Key|Two`
  (bind _keep_playing_ (`self.Keep Playing!`))
  ;[1 1 1] Checking Strings
  (:`Pressed`
    (`GameplayStatics.PlaySoundAttached` "/Game/Props/Blueprints/2.2" (`self.String1`))
    (if (`KismetStringLibrary.EqualEqual_StrStr` (`self.Solution`) (`self.PlaySolution`))
      (set `self.Solved?` true)
      (else
        (set `self.PlaySolution` (`KismetStringLibrary.Concat_StrStr` (`self.PlaySolution`) (`self.D`)))
        (`SceneComponent.ToggleVisibility` _keep_playing_ false)
        (`KismetSystemLibrary.Delay` 0.5)
        (`SceneComponent.ToggleVisibility` _keep_playing_ false)
        (goto _label)))))

(event `Key|Three`
  (bind _keep_playing_ (`self.Keep Playing!`))
  ;[1 1 1] Checking Strings
  (:`Pressed`
    (`GameplayStatics.PlaySoundAttached` "/Game/Props/Blueprints/3.3" (`self.String1`))
    (if (`KismetStringLibrary.EqualEqual_StrStr` (`self.Solution`) (`self.PlaySolution`))
      (set `self.Solved?` true)
      (else
        (set `self.PlaySolution` (`KismetStringLibrary.Concat_StrStr` (`self.PlaySolution`) (`self.E`)))
        (`SceneComponent.ToggleVisibility` _keep_playing_ false)
        (`KismetSystemLibrary.Delay` 0.5)
        (`SceneComponent.ToggleVisibility` _keep_playing_ false)
        (goto _label)))))

(event `self.Box1.OnComponentBeginOverlap`
  (params (OtherActor :type "Actor Object Reference") (OtherComp :type "PrimitiveComponent Object Reference") (OtherBodyIndex :type Integer))
  (bind _returnvalue (`GameplayStatics.GetPlayerController` 0))
  (if (`self.Solved?`)
    (`|ExecutionSequence`
      (:`then_0`
        _)
      (:`then_1`
        _))
    (`self.DisableInput` _returnvalue :!label _label_3)
    (else
      (set `self.HarpMode` true)
      (`self.EnableInput` _returnvalue)))
  (`SceneComponent.ToggleVisibility` (`self.HelpText`) false))

(event `Key|Four`
  (bind _keep_playing_ (`self.Keep Playing!`))
  ;[1 1 1] Checking Strings
  (:`Pressed`
    (`GameplayStatics.PlaySoundAttached` "/Game/Props/Blueprints/4.4" (`self.String1`))
    (if (`KismetStringLibrary.EqualEqual_StrStr` (`self.Solution`) (`self.PlaySolution`))
      (set `self.Solved?` true)
      (else
        (set `self.PlaySolution` (`KismetStringLibrary.Concat_StrStr` (`self.PlaySolution`) (`self.F`)))
        (`SceneComponent.ToggleVisibility` _keep_playing_ false)
        (`KismetSystemLibrary.Delay` 0.5)
        (`SceneComponent.ToggleVisibility` _keep_playing_ false)
        (goto _label)))))

(event `self.Box1.OnComponentEndOverlap`
  (params (OtherActor :type "Actor Object Reference") (OtherComp :type "PrimitiveComponent Object Reference") (OtherBodyIndex :type Integer))
  (goto _label_3))

(event `Key|Five`
  (bind _keep_playing_ (`self.Keep Playing!`))
  ;[1 1 1] Checking Strings
  (:`Pressed`
    (`GameplayStatics.PlaySoundAttached` "/Game/Props/Blueprints/5.5" (`self.String1`))
    (if (`KismetStringLibrary.EqualEqual_StrStr` (`self.Solution`) (`self.PlaySolution`))
      (set `self.Solved?` true)
      (else
        (set `self.PlaySolution` (`KismetStringLibrary.Concat_StrStr` (`self.PlaySolution`) (`self.G`)))
        (`SceneComponent.ToggleVisibility` _keep_playing_ false)
        (`KismetSystemLibrary.Delay` 0.5)
        (`SceneComponent.ToggleVisibility` _keep_playing_ false)
        (goto _label)))))

(event `Key|Six`
  (bind _keep_playing_ (`self.Keep Playing!`))
  ;[1 1 1] Checking Strings
  (:`Pressed`
    (`GameplayStatics.PlaySoundAttached` "/Game/Props/Blueprints/6.6" (`self.String1`))
    (if (`KismetStringLibrary.EqualEqual_StrStr` (`self.Solution`) (`self.PlaySolution`))
      (set `self.Solved?` true)
      (else
        (set `self.PlaySolution` (`KismetStringLibrary.Concat_StrStr` (`self.PlaySolution`) (`self.A`)))
        (`SceneComponent.ToggleVisibility` _keep_playing_ false)
        (`KismetSystemLibrary.Delay` 0.5)
        (`SceneComponent.ToggleVisibility` _keep_playing_ false)
        (goto _label)))))

(event `Key|Seven`
  (bind _keep_playing_ (`self.Keep Playing!`))
  ;[1 1 1] Checking Strings
  (:`Pressed`
    (`GameplayStatics.PlaySoundAttached` "/Game/Props/Blueprints/7.7" (`self.String1`))
    (if (`KismetStringLibrary.EqualEqual_StrStr` (`self.Solution`) (`self.PlaySolution`))
      (set `self.Solved?` true)
      (else
        (set `self.PlaySolution` (`KismetStringLibrary.Concat_StrStr` (`self.PlaySolution`) (`self.B`)))
        (`SceneComponent.ToggleVisibility` _keep_playing_ false)
        (`KismetSystemLibrary.Delay` 0.5)
        (`SceneComponent.ToggleVisibility` _keep_playing_ false)
        (goto _label)))))

(fn `NewFunction`
  (set `self.HarpCam` (`self.HarpCam`))
  (`AddComponent|CameraComponent_95`))

(fn `UserConstructionScript`)