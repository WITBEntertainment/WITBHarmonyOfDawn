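; HUD Blueprint that draws the inventory menu and first-person crosshair with materials on each DrawHUD.
; While MyCharacter's menu is open, it draws the menu panel, a bow icon if the inventory reference allows equipping one, and a cursor at the mouse position.
; Otherwise, in first person, it draws the crosshair from the viewport's half-size point.
; The cursor reuses the crosshair material, and all elements use fixed pixel sizes.
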(event `self.ReceiveDrawHUD`
  (params (SizeX :type Integer) (SizeY :type Integer))
  (bind _returnvalue (/ 600.0 2.0))
  (bind (_locationx _locationy) (`PlayerController.GetMousePosition` (`GameplayStatics.GetPlayerController` 0)))
  (bind (_sizex _sizey) (`PlayerController.GetViewportSize` (`GameplayStatics.GetPlayerController` 0)))
  (bind (_sizex_2 _sizey_2) (`PlayerController.GetViewportSize` (`GameplayStatics.GetPlayerController` 0)))
  (bind _returnvalue_2 (- _returnvalue (/ (`KismetMathLibrary.Conv_IntToDouble` (- SizeY _sizey)) 2.0)))
  (bind _returnvalue_3 (- _returnvalue (/ (`KismetMathLibrary.Conv_IntToDouble` (- SizeX _sizex)) 2.0)))
  ;[1 1 1] InventoryMenu
  (bind _asmycharacter_c (cast `/Game/Blueprints/MyCharacter` (`GameplayStatics.GetPlayerCharacter` 0)))
  (if (`/Game/Blueprints/MyCharacter.isMenuOpen` _asmycharacter_c)
    (`|ExecutionSequence`
      (:`then_0`
        (`self.DrawMaterial` "/Game/Tools/UIElements/menu_Mat.menu_Mat" _returnvalue_3 _returnvalue_2 600.0 600.0 0.0 0.0 1.0 1.0))
      (:`then_1`
        (if (`/Game/Blueprints/inventory.CanEquipBow` (`self.INventoryRef`))
          (`self.DrawMaterialSimple` "/Game/Tools/UIElements/BOW_Mat.BOW_Mat" _returnvalue_3 _returnvalue_2 100.0 100.0)))
      (:`then_6`
        ;;[1 1 1] MouseCursor
        (`self.DrawMaterialSimple` "/Game/Tools/Spinnerette/crossHairs_Mat.crossHairs_Mat" _locationx _locationy 32.0 32.0)))
    (else
      ;[1 1 1] DrawCrossHairs
      (bind _asmycharacter_c_2 (cast `/Game/Blueprints/MyCharacter` (`GameplayStatics.GetPlayerCharacter` 0)))
      (if (`/Game/Blueprints/MyCharacter.firstPerson` _asmycharacter_c_2)
        (`self.DrawMaterial` "/Game/Tools/Spinnerette/crossHairs_Mat.crossHairs_Mat" (/ (`KismetMathLibrary.Conv_IntToDouble` _sizex_2) 2.0) (/ (`KismetMathLibrary.Conv_IntToDouble` _sizey_2) 2.0) 32.0 32.0 0.0 0.0 1.0 1.0)))))

(fn `UserConstructionScript`)