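; Inventory Blueprint that tracks which items are available to equip: spinner, lung, mallet and bow.
; On BeginPlay, a sequence sets each item's can-equip flag from its matching ownership flag.
; It then searches an array for the currently equipped value when that value is not "None", breaking on a match without acting on it.
; The construction script is empty.
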(event `self.ReceiveBeginPlay`
  (`|ExecutionSequence`
    (:`then_0`
      (if (`self.Has_Spinner`)
        (set `self.CanEquipSpin` true)
        (else
          (set `self.CanEquipSpin` false))))
    (:`then_1`
      (if (`self.Has_Lung`)
        (set `self.CanEquipLung` true)
        (else
          (set `self.CanEquipLung` false))))
    (:`then_2`
      (if (`self.Has_Mallet`)
        (set `self.CanEquipMallet` true)
        (else
          (set `self.CanEquipMallet` false))))
    (:`then_3`
      (if (`self.HasBow`)
        (set `self.CanEquipBow` true)
        (else
          (set `self.CanEquipBow` false))))
    (:`then_4`
      (if (`KismetStringLibrary.NotEqual_StrStr` (`self.CurrentlyEquiped`))
        (for _array_element (`self.CurrentlyEquipValue`)
          (if (`KismetStringLibrary.EqualEqual_StrStr` _array_element (`self.CurrentlyEquiped`))
            (break)))))))

(fn `UserConstructionScript`)